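; Base enemy character for a hack-and-slash game, handling AI combat, health and death, with a boss option that ends the game.
; Pawn sensing starts looping chase and turn logic, triggering random montage attacks on a cooldown.
; Swing events toggle weapon overlap, with an array limiting damage to one hit per swing.
; Received damage plays hit reactions or death, which notifies a gate, while a timer keeps the HP bar facing the camera.
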(event Custom|Check%20HP%20Widget
  (bind _hpwidget (Variables|Default|GetHPWidget))
  (bind _hpwidget_2 (Variables|Default|GetHPWidget))
  ;[1 1 1] Show/Hide/Rotate HP Bar
  (if (Variables|Default|GetReadyToFight?)
    (if (Variables|Default|GetDead?)
      (Development|SetHiddeninGame _hpwidget true false)
      (else
        (Development|SetHiddeninGame _hpwidget false false)
        (bind _asthird_person_character (Utilities|Casting|CastToBP_ThirdPersonCharacter (Game|GetPlayerCharacter 0)))
        (Transformation|SetWorldRotation _hpwidget_2 (Math|Rotator|MakeRotator 0.0 0.0 (.yaw (Math|Rotator|FindLookatRotation (Transformation|GetWorldLocation _hpwidget_2) (Transformation|GetWorldLocation (Variables|/Game/HackAndSlash/MainCharacter/Blueprints/BP_ThirdPersonCharacter.BP_ThirdPersonCharacter_C|GetFollowCamera _asthird_person_character))))) false false)))))

(event EventBeginPlay
  ;[1 1 1] Create HP Bar
  (bind _aswbp_enemy_hp (Utilities|Casting|CastToWBP_EnemyHP (UserInterface|GetUserWidgetObject (Variables|Default|GetHPWidget))))
  (Variables|/Game/HackAndSlash/Enemies/BasicEnemy/Widgets/WBP_EnemyHP.WBP_EnemyHP_C|SetEnemyReference _aswbp_enemy_hp self)
  (Utilities|Time|SetTimerbyEvent (delegate Custom|Check%20HP%20Widget) 0.05 true))

(event Custom|Receive%20Damage
  (params (Damage :type Float%20%28single-precision%29) (AttackType :type E_AttackTypes%20Enum :default "NewEnumerator0"))
  ;[1 1 1] Receive Damage Event
  (if (Variables|Default|GetReadyToFight?)
    (if (not (Variables|Default|GetDead?))
      (bind _output_get (Variables|Default|SetCurrentHP (- (Variables|Default|GetCurrentHP) Damage)))
      ;[1 1 1] Detect Death
      (if (<= _output_get 0.0)
        (CallFunction|EnemyDeath)
        (else
          (switch Utilities|FlowControl|Switch|SwitchonE_AttackTypes AttackType
            (:NewEnumerator0
              _)
            (:NewEnumerator1
              _)
            (:NewEnumerator2
              _))
          (Animation|PlayAnimMontage "/Game/HackAndSlash/Enemies/BasicEnemy/Animations/HitReact_Front_Montage.HitReact_Front_Montage" 0.5 "None"))))))

(event Custom|Enemy%20Death
  (bind _gatereference (Variables|Default|GetGateReference))
  ;[1 1 1] Death Event
  (Variables|Default|SetDead? true)
  (Variables|Default|SetReadyToFight? false)
  (Variables|/Script/AIModule.PawnSensingComponent|SetbSeePawns (Variables|Default|GetPawnSensing) false)
  (Development|SetHiddeninGame (Variables|Default|GetHPWidget) true false)
  (Components|Animation|PlayAnimation (Variables|Character|GetMesh) (Variables|Default|GetDeathAnimation) false)
  (Components|Movement|StopMovementImmediately (Variables|Character|GetCharacterMovement))
  (Utilities|IsValid _gatereference
    (:Is%20Valid
      (Default|CountEnemies _gatereference self))
    (:Is%20Not%20Valid
      _))
  (Utilities|FlowControl|Delay 3.0)
  (if (Variables|Default|GetBoss?)
    (CallFunction|GameFinished)
    (else
      (Actor|DestroyActor))))

(event Custom|Game%20Finished
  (bind _returnvalue (Game|GetPlayerController 0))
  ;[1 1 1] Show Game Over Widget When Boss Dies. Logic is here because we need access to Enemy Death logic above.
  (bind _returnvalue_2 (UserInterface|CreateWidget "/Game/HackAndSlash/Enemies/Boss/Widgets/WBP_GameFinished.WBP_GameFinished_C"))
  (UserInterface|Viewport|AddtoViewport _returnvalue_2 0)
  (Input|SetInputModeGameandUI _returnvalue _returnvalue_2 "DoNotLock" true)
  (Variables|/Script/Engine.PlayerController|SetbShowMouseCursor _returnvalue true)
  (if (not (Variables|Default|GetBoss?))
    (Actor|DestroyActor)))

(event OnSeePawn(PawnSensing)
  (params (Pawn :type Pawn%20Object%20Reference))
  ;[1 1 1] Target Detection
  (bind _asthird_person_character (Utilities|Casting|CastToBP_ThirdPersonCharacter Pawn))
  (Utilities|FlowControl|Sequence
    (:then_0
      (Utilities|FlowControl|DoOnce false
        (:Completed
          (Variables|Default|SetReadyToFight? true))))
    (:then_1
      (Variables|Default|SetPlayerReference _asthird_person_character)
      (if (not (or (Variables|Default|GetDead?) (Variables|/Game/HackAndSlash/MainCharacter/Blueprints/BP_ThirdPersonCharacter.BP_ThirdPersonCharacter_C|GetDead? (Variables|Default|GetPlayerReference)))) :!label _label
        (CallFunction|LookatTarget)
        (AI|AIMoveTo self "0, 0, 0" (Variables|Default|GetPlayerReference) 1e+02 false
          (:then
            (Utilities|FlowControl|Delay 0.2)
            (goto _label))
          (:OnSuccess
            ;[1 1 1] Attacks & Animations
            (if (not (or (Class|AnimInstance|IsAnyMontagePlaying (Components|SkeletalMesh|GetAnimInstance (Variables|Character|GetMesh))) (Variables|Default|GetAttacking?)))
              (Variables|Default|SetAttacking? true)
              (if (not (or (Variables|Default|GetDead?) (Variables|/Game/HackAndSlash/MainCharacter/Blueprints/BP_ThirdPersonCharacter.BP_ThirdPersonCharacter_C|GetDead? (Variables|Default|GetPlayerReference))))
                (switch int (Math|Random|RandomInteger 2)
                  (:0
                    (Animation|PlayAnimMontage "/Game/HackAndSlash/Enemies/BasicEnemy/Animations/Attack_A_Montage.Attack_A_Montage" 1.0 "None"))
                  (:1
                    (Animation|PlayAnimMontage "/Game/HackAndSlash/Enemies/BasicEnemy/Animations/Attack_C_Montage.Attack_C_Montage" 1.0 "None")))
                (Utilities|FlowControl|Delay (Variables|Default|GetBasicAttackCooldown))
                (Variables|Default|SetAttacking? false)))))))))

(event OnComponentBeginOverlap(WeaponCollision)
  (params (OverlappedComponent :type Primitive%20Component%20Object%20Reference) (OtherActor :type Actor%20Object%20Reference) (OtherComp :type Primitive%20Component%20Object%20Reference) (OtherBodyIndex :type Integer) (bFromSweep :type Boolean) (SweepResult :type Hit%20Result%20Structure%20%28by%20ref%29))
  (bind _playerrefarray (Variables|Default|GetPlayerRefArray))
  ;[1 1 1] Attack Damage (Outgoing)
  (bind _asthird_person_character (Utilities|Casting|CastToBP_ThirdPersonCharacter OtherActor))
  (if (not (Utilities|Array|ContainsItem _playerrefarray _asthird_person_character))
    (Utilities|Array|AddUnique _playerrefarray 0)
    (Default|MainCharacterReceivedDamage _asthird_person_character 1e+01 "NewEnumerator0" (Transformation|GetActorLocation))))

(event Custom|Look%20At%20Target
  ;[1 1 1] Target Acquisition
  (Utilities|FlowControl|DoOnce false
    (:Completed
      (if (not (Variables|Default|GetDead?)) :!label _label
        (Transformation|SetActorRotation (Math|Rotator|MakeRotator 0.0 0.0 (.yaw (Math|Interpolation|RInterpTo (Transformation|GetActorRotation) (Math|Rotator|FindLookatRotation (Transformation|GetActorLocation) (Transformation|GetActorLocation (Variables|Default|GetPlayerReference))) (Utilities|Time|GetWorldDeltaSeconds) 3.0))))
        (Utilities|FlowControl|Delay 0.1)
        (goto _label)))))

(event Custom|Enemy%20Swing%20Start
  ;[1 1 1] Swing System
  (Collision|SetCollisionResponsetoChannel (Variables|Default|GetWeaponCollision) "ECC_PhysicsBody" "ECR_Overlap"))

(event Custom|Enemy%20Swing%20End
  ;[1 1 1] Swing System
  (Utilities|Array|Clear (Variables|Default|GetPlayerRefArray))
  (Collision|SetCollisionResponsetoChannel (Variables|Default|GetWeaponCollision) "ECC_PhysicsBody" "ECR_Ignore"))

(fn ConstructionScript)