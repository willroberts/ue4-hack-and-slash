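; Homing missile projectile for the hack-and-slash main character that seeks enemies and destroys itself after a fixed lifetime.
; A looping timer starts on spawn alongside the targeting logic, which replaces a missing or dead homing target with a random living, fight-ready enemy from a shuffled list.
; Sphere overlaps damage living enemies and spawn an impact effect without destroying the missile, so it can hit repeatedly.
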(event OnComponentBeginOverlap(SphereCollision)
  (params (OverlappedComponent :type Primitive%20Component%20Object%20Reference) (OtherActor :type Actor%20Object%20Reference) (OtherComp :type Primitive%20Component%20Object%20Reference) (OtherBodyIndex :type Integer) (bFromSweep :type Boolean) (SweepResult :type Hit%20Result%20Structure%20%28by%20ref%29))
  ;[1 1 1] Homing Projectile Collision and Damage
  (bind _asbp_enemy_base (Utilities|Casting|CastToBP_Enemy_Base OtherActor))
  (if (not (Variables|/Game/HackAndSlash/Enemies/BasicEnemy/Blueprints/BP_Enemy_Base.BP_Enemy_Base_C|GetDead? _asbp_enemy_base))
    (Default|ReceiveDamage _asbp_enemy_base 5e+01 "NewEnumerator0")
    (Effects|SpawnEmitteratLocation 0 "0, 0, 0")))

(event Custom|Enemy%20Ready%20to%20Follow
  ;[1 1 1] Homing Projectile Targeting
  (Utilities|IsValid (Variables|/Script/Engine.ProjectileMovementComponent|GetHomingTargetComponent (Variables|Default|GetProjectileMovement))
    (:Is%20Valid
      (bind _asbp_enemy_base (Utilities|Casting|CastToBP_Enemy_Base (Components|GetOwner (Variables|/Script/Engine.ProjectileMovementComponent|GetHomingTargetComponent (Variables|Default|GetProjectileMovement)))))
      (if (Variables|/Game/HackAndSlash/Enemies/BasicEnemy/Blueprints/BP_Enemy_Base.BP_Enemy_Base_C|GetDead? _asbp_enemy_base)
        (Variables|/Script/Engine.ProjectileMovementComponent|SetHomingTargetComponent (Variables|Default|GetProjectileMovement) 0)
        (bind _outactors (Actor|GetAllActorsOfClass "/Game/HackAndSlash/Enemies/BasicEnemy/Blueprints/BP_Enemy_Base.BP_Enemy_Base_C" :!label _label))
        (Utilities|Array|Shuffle _outactors)
        (bind _array_element (Utilities|Array|ForEachLoopwithBreak _outactors :!label _label_2)
          (:LoopBody
            (if (and (Variables|/Game/HackAndSlash/Enemies/BasicEnemy/Blueprints/BP_Enemy_Base.BP_Enemy_Base_C|GetReadyToFight? _array_element) (not (Variables|/Game/HackAndSlash/Enemies/BasicEnemy/Blueprints/BP_Enemy_Base.BP_Enemy_Base_C|GetDead? _array_element)))
              (Variables|/Script/Engine.ProjectileMovementComponent|SetHomingTargetComponent (Variables|Default|GetProjectileMovement) (Variables|/Script/Engine.Character|GetCapsuleComponent _array_element))
              (goto _label_2 Break))))))
    (:Is%20Not%20Valid
      (goto _label))))

(event EventBeginPlay
  ;[1 1 1] Queue Projectile Destruction When Spawned
  (Utilities|Time|SetTimerbyEvent (EventDispatchers|CreateEvent :!event Custom|Enemy%20Ready%20to%20Follow) 1.0 true)
  (Utilities|FlowControl|Delay 2e+01)
  (Actor|DestroyActor))

(fn ConstructionScript)