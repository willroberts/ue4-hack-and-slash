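; Level gate that opens once every enemy in its EnemyReference list has been removed.
; On BeginPlay it hands itself to each listed enemy as GateReference.
; CountEnemies removes the passed enemy from the list and triggers OpenGate when the list is empty.
; OpenGate slides GateMesh to a lowered relative Z with an eased, timed MoveComponentTo, keeping its X, Y and rotation.
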(event Custom|Count%20Enemies
  (params (Item :type BP%20Enemy%20Base%20Object%20Reference%20%28by%20ref%29))
  (bind _enemyreference (Variables|Default|GetEnemyReference))
  ;[1 1 1] Count Enemy References
  (Utilities|Array|RemoveItem _enemyreference Item)
  (if (== (Utilities|Array|Length _enemyreference) 0)
    (CallFunction|OpenGate)))

(event Custom|Open%20Gate
  (bind _gatemesh (Variables|Default|GetGateMesh))
  (bind _relativelocation (Variables|/Script/Engine.SceneComponent|GetRelativeLocation _gatemesh))
  ;[1 1 1] Open Gate
  (Components|MoveComponentTo _gatemesh (Math|Vector|MakeVector (.x _relativelocation) (.y _relativelocation) -6e+02) (Variables|/Script/Engine.SceneComponent|GetRelativeRotation _gatemesh) true true 3.0 false))

(event EventBeginPlay
  ;[1 1 1] Add Enemy References
  (for _array_element (Variables|Default|GetEnemyReference)
    (Variables|/Game/HackAndSlash/Enemies/BasicEnemy/Blueprints/BP_Enemy_Base.BP_Enemy_Base_C|SetGateReference _array_element self)))

(fn ConstructionScript)