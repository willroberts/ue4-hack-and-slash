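; BP_Pickup_Ultimate is an interactable pickup that readies the player character's ultimate skill.
; Overlapping the collision enables input and shows an interaction prompt; pressing F sets the skill ready and hides the pickup.
; Ending overlap always disables input, shows an ultimate-skill tooltip, then destroys the actor after a delay, whether or not F was pressed.
; A self-restarting timeline floats the particle system vertically.
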(event OnComponentBeginOverlap(Pickup_Collision)
  (params (OverlappedComponent :type Primitive%20Component%20Object%20Reference) (OtherActor :type Actor%20Object%20Reference) (OtherComp :type Primitive%20Component%20Object%20Reference) (OtherBodyIndex :type Integer) (bFromSweep :type Boolean) (SweepResult :type Hit%20Result%20Structure%20%28by%20ref%29))
  ;[1 1 1] Pickup Interaction Begin
  (Utilities|Casting|CastToThirdPersonCharacter OtherActor)
  (Input|EnableInput (Game|GetPlayerController 0))
  (bind _returnvalue (UserInterface|CreateWidget "/Game/HackAndSlash/Pickups/WBP_InteractionMessage.WBP_InteractionMessage_C" 0 "Press \"F\" To Interact"))
  (bind _output_get (Variables|Default|SetMessageReference _returnvalue))
  (UserInterface|Viewport|AddtoViewport _output_get 0))

(event OnComponentEndOverlap(Pickup_Collision)
  (params (OverlappedComponent :type Primitive%20Component%20Object%20Reference) (OtherActor :type Actor%20Object%20Reference) (OtherComp :type Primitive%20Component%20Object%20Reference) (OtherBodyIndex :type Integer))
  ;[1 1 1] Pickup Interaction End
  (Utilities|Casting|CastToThirdPersonCharacter OtherActor)
  (Input|DisableInput (Game|GetPlayerController 0))
  (Widget|RemovefromParent (Variables|Default|GetMessageReference))
  ;[1 1 1] Ultimate Skill Tooltip
  (bind _returnvalue (UserInterface|CreateWidget "/Game/HackAndSlash/Pickups/WBP_InteractionMessage.WBP_InteractionMessage_C" 0 "Press \"E\" to  use your Ultimate Skill!"))
  (bind _output_get (Variables|Default|SetMessageReference _returnvalue))
  (UserInterface|Viewport|AddtoViewport _output_get 0)
  (Utilities|FlowControl|Delay 6.0)
  (Widget|RemovefromParent (Variables|Default|GetMessageReference))
  (Actor|DestroyActor))

(event Custom|Start%20Transform
  ;[1 1 1] Start Transform
  (bind _asthird_person_character (Utilities|Casting|CastToThirdPersonCharacter (Game|GetPlayerCharacter 0)))
  (Default|UltimateSkillReady _asthird_person_character true)
  (Widget|RemovefromParent (Variables|Default|GetMessageReference))
  (Rendering|SetActorHiddenInGame true))

(event Custom|Floating
  (bind _particlesystem (Variables|Default|GetParticleSystem))
  (bind _relativelocation (Variables|/Script/Engine.SceneComponent|GetRelativeLocation _particlesystem))
  ;[1 1 1] Floating Effect
  (bind _floatingcurve (Timeline|Floating%20Timeline PlayFromStart)
    (:Update
      (Transformation|SetRelativeLocation _particlesystem (Math|Vector|MakeVector (.x _relativelocation) (.y _relativelocation) _floatingcurve) false false))
    (:Finished
      (Utilities|FlowControl|Delay 0.1)
      (CallFunction|Floating))))

(event EventBeginPlay
  ;[1 1 1] Floating Effect
  (CallFunction|Floating))

(event Input|KeyboardEvents|F
  (params (Key :type Key%20Structure))
  ;[1 1 1] Start Transform
  (:Pressed
    (CallFunction|StartTransform)))

(fn ConstructionScript)